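; Player character Blueprint handling movement, look, pausing and world interaction.
; Sprint is speed-gated, crouch uses a timeline to blend capsule height and walk speed with server/client events, and ladders switch movement to Flying along the up vector.
; Look applies invert settings from DR_GameInstance and derives spine rotation from pitch.
; Interact input sets ladder and interactable flags, while Primary Fire line-traces from the camera to use security panel keypads.
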(event `InputAction|Interactions`
  (params (Key :type "Key Structure"))
  ;[1 1 1] Ladder movements
  (:`Pressed`
    (if (`self.Is Near Ladder`)
      (set `self.Is On Ladder` true))))

(event `InputAction|Interactions`
  (params (Key :type "Key Structure"))
  ;[1 1 1] Dealing with Interactables
  (:`Pressed`
    (if (`self.Is Near Interactable`)
      (set `self.Activate Interactable` true))))

(event `InputAction|Pause`
  (params (Key :type "Key Structure"))
  ;[1 1 1] Setting the Pause Menu on the game
  (:`Pressed`
    (if (not (`self.Is Paused?`))
      (bind _returnvalue (`|CreateWidget` "/Game/BluePrints/UserInterfaces/DR_Pause_Menu.DR_Pause_Menu_C"))
      (`UserWidget.AddToViewport` _returnvalue 0)
      (`WidgetBlueprintLibrary.SetInputMode_GameAndUIEx` (`GameplayStatics.GetPlayerController` 0) _returnvalue)
      (set `self.Is Paused?` true))))

(event `Set Player Spine Rotation`
  (bind (_returnvalue_roll _returnvalue_pitch) (`KismetMathLibrary.BreakRotator` (`self.GetControlRotation`)))
  ;[1 1 1] Dealing with Mesh rotation
  (set `self.Spine Rotation` (`KismetMathLibrary.MakeRotator` (`KismetMathLibrary.SelectFloat` (- 360.0 _returnvalue_pitch) (* _returnvalue_pitch -1.0) (> _returnvalue_pitch 180.0)))))

(event `InputAxis|Forwards_Backwards`
  (params (AxisValue :type "Float (single-precision)"))
  (bind (_velocity_x _velocity_y) (`KismetMathLibrary.BreakVector` (`MovementComponent.Velocity` (`self.CharacterMovement`))))
  ;[1 1 1] Character Walk/Run Movement
  ;[1 1 1] Ladder movements
  (if (`self.Is On Ladder`)
    (`CharacterMovementComponent.SetMovementMode` (`self.CharacterMovement`) "MOVE_Flying" 0)
    (`self.AddMovementInput` (`self.GetActorUpVector` (`GameplayStatics.GetPlayerCharacter` 0)) AxisValue)
    (else
      (`self.AddMovementInput` (`KismetMathLibrary.GetForwardVector` (`self.K2_GetActorRotation`)) AxisValue)
      (if (and (`self.IsSprinting?`) (< (`KismetMathLibrary.VSize` (`KismetMathLibrary.MakeVector` _velocity_x _velocity_y)) (+ (`self.Character_StandingMovementSpeed`) (* (- (`self.Character_RunMovementSpeed`) (`self.Character_StandingMovementSpeed`)) 0.8))))
        (`self.SetSprinting` false)))))

(event `InputAxis|Left_Right`
  (params (AxisValue :type "Float (single-precision)"))
  ;[1 1 1] Character Walk/Run Movement
  (if (not (`self.Is On Ladder`))
    (`self.AddMovementInput` (`KismetMathLibrary.GetRightVector` (`self.K2_GetActorRotation`)) AxisValue)))

(event `InputAction|Crouch`
  (params (Key :type "Key Structure"))
  ;[1 1 1] Character Crouching
  (:`Pressed`
    (`self.Crouch_Player`)))

(event `Crouch_Player`
  ;[1 1 1] Character Crouching
  (`/Engine/EditorBlueprintResources/ActorMacros.Switch Has Authority`
    (:`Authority`
      _)
    (:`Remote`
      (`self.Crouch_Client`)))
  (`self.Crouch_Server`))

(event `InputAction|Jump`
  (params (Key :type "Key Structure"))
  ;[1 1 1] Character Jumping
  (:`Pressed`
    (if (`self.IsCrouched?`)
      (`self.Crouch_Player`)
      (else
        (`self.Jump`)))))

(event `InputAction|Sprint_GamePad`
  (params (Key :type "Key Structure"))
  ;[1 1 1] Character Walk/Run Movement
  (:`Pressed`
    (if (`self.IsCrouched?`) :!label _label
      (`self.Crouch_Player`)
      (else
        (`self.SetSprinting` true))))
  (:`Released`
    (`self.SetSprinting` false :!label _label_2)))

(event `InputAction|Sprint_Keyboard`
  (params (Key :type "Key Structure"))
  ;[1 1 1] Character Walk/Run Movement
  (:`Pressed`
    (goto _label))
  (:`Released`
    (goto _label_2)))

(event `Crouch_Server`
  ;[1 1 1] Character Crouching
  (bind _output_get (set `self.IsCrouched?` (not (`self.IsCrouched?`)) :!label _label_3))
  (if _output_get
    (bind (_direction _height) (`Timeline|Crouch_Animation` :!label _label_4)
      (:`Update`
        (`CapsuleComponent.SetCapsuleHalfHeight` (`self.CapsuleComponent`) (`KismetMathLibrary.Lerp` (`self.Character_Standing`) (`self.Character_Crouch`) _height) true)
        (set `CharacterMovementComponent.MaxWalkSpeed` (`KismetMathLibrary.Lerp` (`self.Character_StandingMovementSpeed`) (`self.Character_CrouchMovementSpeed`) _height) (`self.CharacterMovement`))))
    (else
      (goto _label_4 :!via `Reverse`))))

(event `InputAxis|Look Up_Down`
  (params (AxisValue :type "Float (single-precision)"))
  ;[1 1 1] Character Look
  (if (`self.Is Invert Y?`)
    (`/Engine/EditorBlueprintResources/StandardMacros.NegateFloat` AxisValue
      (:`  `
        _)))
  (`self.AddControllerPitchInput` AxisValue)
  ;[1 1 1] Character Crouching
  (`self.Set Player Spine Rotation`))

(event `Crouch_Client`
  ;[1 1 1] Character Crouching
  (goto _label_3))

(event `SetSprinting`
  (params (`Sprinting?` :type Boolean))
  (bind (_velocity_x _velocity_y) (`KismetMathLibrary.BreakVector` (`MovementComponent.Velocity` (`self.CharacterMovement`))))
  ;[1 1 1] Character Walk/Run Movement
  (if `Sprinting?`
    (if (>= (`KismetMathLibrary.VSize` (`KismetMathLibrary.MakeVector` _velocity_x _velocity_y)) (* (`self.Character_StandingMovementSpeed`) 0.75))
      (set `CharacterMovementComponent.MaxWalkSpeed` (`self.Character_RunMovementSpeed`) (`self.CharacterMovement`))
      (`KismetSystemLibrary.Delay` 0.3)
      (set `self.IsSprinting?` true))
    (else
      (set `CharacterMovementComponent.MaxWalkSpeed` (`self.Character_StandingMovementSpeed`) (`self.CharacterMovement`))
      (set `self.IsSprinting?` false))))

(event `InputAxis|Look Left_Right`
  (params (AxisValue :type "Float (single-precision)"))
  ;[1 1 1] Character Look
  (if (`self.Is Invert X?`)
    (`/Engine/EditorBlueprintResources/StandardMacros.NegateFloat` AxisValue
      (:`  `
        _)))
  (`self.AddControllerYawInput` AxisValue))

(event `self.ReceivePossessed`
  (params (NewController :type "Controller Object Reference"))
  ;[1 1 1] Setting with Inverted Controls
  (bind _asdr_game_instance (cast `/Game/BluePrints/Game_Settings/DR_GameInstance` (`GameplayStatics.GetGameInstance`))
    (:`then`
      (set `self.Is Invert Y?` (`/Game/BluePrints/Game_Settings/DR_GameInstance.Inverted Y` _asdr_game_instance))
      (set `self.Is Invert X?` (`/Game/BluePrints/Game_Settings/DR_GameInstance.Inverted X` _asdr_game_instance)))
    (:`CastFailed`
      (`KismetSystemLibrary.PrintString` "I didn't work. dummy"))))

(event `InputAction|Primary Fire`
  (params (Key :type "Key Structure"))
  (bind _camera (`self.Camera`))
  (bind _returnvalue (`SceneComponent.K2_GetComponentLocation` _camera))
  (:`Pressed`
    (`KismetSystemLibrary.PrintString` "shooot")
    (bind (_outhit _returnvalue_2) (`KismetSystemLibrary.LineTraceSingle` :`Start` _returnvalue :`End` (+ _returnvalue (* (`SceneComponent.GetForwardVector` _camera) (`self.Interaction Distance`))) :`TraceChannel` "TraceTypeQuery1" :`DrawDebugType` "ForDuration"))
    (if _returnvalue_2
      (bind _asbp_security_panel (cast `/Game/BluePrints/Interactables/BP_SecurityPanel` (`.HitActor` (`GameplayStatics.BreakHitResult` _outhit))))
      (`/Game/BluePrints/Interactables/BP_SecurityPanel.Use Keypad` _asbp_security_panel))))

(fn `UserConstructionScript`)