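; Player controller for gamepad support that forwards D-pad presses to the main menu widget as navigation requests.
; Each D-pad direction calls RecieveNavigationRequest on MainWidget with its own enum value, and Up also prints a debug string.
; The code that creates the DR_WB_Main_Menu widget, shows the cursor and sets Game and UI input is disconnected, so MainWidget is never assigned here and BeginPlay is empty.
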(event `Key|Gamepad_DPad_Right`
  (params (Key :type "Key Structure"))
  (:`Pressed`
    (`/Game/BluePrints/UserInterfaces/MainMenu_Widgets/DR_WB_Main_Menu.RecieveNavigationRequest` (`self.Main Widget`) "NewEnumerator3")))

(event `self.ReceiveBeginPlay`
  ;[1 1 1] Need to see if i can put this into the actual widget thingy, or if i need to re work around it.
)

(event `Key|Gamepad_DPad_Left`
  (params (Key :type "Key Structure"))
  (:`Pressed`
    (`/Game/BluePrints/UserInterfaces/MainMenu_Widgets/DR_WB_Main_Menu.RecieveNavigationRequest` (`self.Main Widget`) "NewEnumerator2")))

(event `Key|Gamepad_DPad_Up`
  (params (Key :type "Key Structure"))
  (:`Pressed`
    (`/Game/BluePrints/UserInterfaces/MainMenu_Widgets/DR_WB_Main_Menu.RecieveNavigationRequest` (`self.Main Widget`) "NewEnumerator0")
    (`KismetSystemLibrary.PrintString` "ey")))

(event `Key|Gamepad_DPad_Down`
  (params (Key :type "Key Structure"))
  (:`Pressed`
    (`/Game/BluePrints/UserInterfaces/MainMenu_Widgets/DR_WB_Main_Menu.RecieveNavigationRequest` (`self.Main Widget`) "NewEnumerator1")))

(fn `UserConstructionScript`)