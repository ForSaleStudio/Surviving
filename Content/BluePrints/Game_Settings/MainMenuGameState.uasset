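; Game State for the main menu that stores the current menu state enum.
; Set Menu State fires an On Menu State Changed dispatcher with the new and previous states before storing the new value.
; Get Menu State returns the stored value.
; BeginPlay and both accessors print on-screen debug messages.
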(event `self.ReceiveBeginPlay`
  (`KismetSystemLibrary.PrintString` "MainMenu Game State being called." true true (struct :`R` 0.023159 :`G` 1.0 :`A` 1.0) 5.0))

(fn `Get Menu State`
  (returns (`Menu State` :type "/Game/BluePrints/Game_Settings/MenuState Enum"))
  (`KismetSystemLibrary.PrintString` "MENU STATE IS SET TO GETTING RIGHT NOW" true true (struct :`R` 1.0 :`G` 0.769096 :`A` 1.0) 5.0)
  (return (`self.MenuState`)))

(fn `Set Menu State`
  (params (New :type "/Game/BluePrints/Game_Settings/MenuState Enum" :default "NewEnumerator0"))
  (`self.OnMenuStateChanged` New (`self.MenuState`))
  (bind _output_get (set `self.MenuState` New))
  (`KismetSystemLibrary.PrintString` "Is the current menu state" true true (struct :`G` 0.66 :`B` 1.0 :`A` 1.0) 5.0)
  (`KismetSystemLibrary.PrintString` (`|GetEnumeratorNameAsString` _output_get) true true (struct :`R` 1.0 :`G` 0.696675 :`A` 1.0) 5.0))

(fn `UserConstructionScript`)