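; World pickup for an inventory item, taking its mesh, scale and interact radius from the ItemToAdd class defaults.
; On BeginPlay it rolls a random amount and writes name and amount to its text widget.
; Sphere overlaps maintain the main character's nearby-pickup list, which drives prompt visibility.
; OnPickup adds to the inventory, records any remainder by ID in LootedPickup, and destroys the actor once emptied.
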(event `self.ReceiveBeginPlay`
  (bind _amount_to_add (`self.Random Amount to Add` (`self.Min Amount`) (`self.Max Amount`)))
  (bind _output_get (set `self.Amount` _amount_to_add))
  (`KismetSystemLibrary.PrintString` (`KismetStringLibrary.Conv_IntToString` _output_get))
  (`self.Update Text`))

(event `On Pickup`
  (params (`Character Ref` :type "/Game/BluePrints/Game_Settings/Characters/Main_Characters/DR_Main_Character_base Object Reference"))
  (bind _inventory_ref (`/Game/BluePrints/Game_Settings/Characters/Main_Characters/DR_Main_Character_base.Inventory Ref` `Character Ref`))
  (bind _inventory_ref_2 (`/Game/BluePrints/Game_Settings/Characters/Main_Characters/DR_Main_Character_base.Inventory Ref` `Character Ref`))
  (bind _nearby_pickup_actors (`/Game/BluePrints/Game_Settings/Characters/Main_Characters/DR_Main_Character_base.Nearby Pickup Actors` `Character Ref`))
  (bind _output (`|GetArrayItem` _nearby_pickup_actors))
  ;[1 0.75 0] Adding the item to the inventory, doing the necessary checks through the main character ref.
  (`/Engine/EditorBlueprintResources/StandardMacros.IsValid` _inventory_ref
    (:`Is Valid`
      (bind (_success __rest) (`/Game/BluePrints/Game_Settings/Items/Inventory_System/Blueprints/BP_Inventory.Add Item` _inventory_ref (`self.Item To Add`) (`self.Amount`)))
      (if _success
        (if (> __rest 0)
          (set `self.Amount` __rest)
          (`KismetArrayLibrary.Array_Add` (`/Game/BluePrints/Game_Settings/Items/Inventory_System/Blueprints/BP_Inventory.Looted Pickup` _inventory_ref_2) (make `/Game/BluePrints/Game_Settings/Items/Inventory_System/Blueprints/Structures/S_SavedPickup` (`self.ID`) (`self.Amount`)))
          (`self.Update Text`)
          (else
            (`KismetArrayLibrary.Array_Add` (`/Game/BluePrints/Game_Settings/Items/Inventory_System/Blueprints/BP_Inventory.Looted Pickup` _inventory_ref_2) (make `/Game/BluePrints/Game_Settings/Items/Inventory_System/Blueprints/Structures/S_SavedPickup` (`self.ID`)))
            (`KismetArrayLibrary.Array_RemoveItem` _nearby_pickup_actors self)
            (`/Engine/EditorBlueprintResources/StandardMacros.IsValid` _output
              (:`Is Valid`
                (`SceneComponent.SetVisibility` (`/Game/BluePrints/Game_Settings/Items/Inventory_System/Blueprints/ItemClasses/BP_PickupActor.Pickup Text` _output) true false)
                (`self.K2_DestroyActor`))
              (:`Is Not Valid`
                (`self.K2_DestroyActor`)))))))))

(event `self.Sphere.OnComponentBeginOverlap`
  (params (OverlappedComponent :type "PrimitiveComponent Object Reference") (OtherActor :type "Actor Object Reference") (OtherComp :type "PrimitiveComponent Object Reference") (OtherBodyIndex :type Integer) (bFromSweep :type Boolean) (SweepResult :type "HitResult Structure (by ref)"))
  ;[1 0.75 0] Setting up the Pickup Text and allowing the player to pick it up and add it to the inventory.
  (bind _asdr_main_character_base (cast `/Game/BluePrints/Game_Settings/Characters/Main_Characters/DR_Main_Character_base` OtherActor))
  (bind _nearby_pickup_actors (`/Game/BluePrints/Game_Settings/Characters/Main_Characters/DR_Main_Character_base.Nearby Pickup Actors` _asdr_main_character_base))
  (if (> (`KismetArrayLibrary.Array_Length` _nearby_pickup_actors) 0)
    (`KismetArrayLibrary.Array_Add` _nearby_pickup_actors self)
    (else
      (`SceneComponent.SetVisibility` (`self.Pickup Text`) true false)
      (`KismetArrayLibrary.Array_Add` _nearby_pickup_actors self))))

(event `self.Sphere.OnComponentEndOverlap`
  (params (OverlappedComponent :type "PrimitiveComponent Object Reference") (OtherActor :type "Actor Object Reference") (OtherComp :type "PrimitiveComponent Object Reference") (OtherBodyIndex :type Integer))
  ;[1 0.75 0] Setting up the Pickup Text and allowing the player to pick it up and add it to the inventory.
  (bind _asdr_main_character_base (cast `/Game/BluePrints/Game_Settings/Characters/Main_Characters/DR_Main_Character_base` OtherActor))
  (bind _nearby_pickup_actors (`/Game/BluePrints/Game_Settings/Characters/Main_Characters/DR_Main_Character_base.Nearby Pickup Actors` _asdr_main_character_base))
  (bind _output (`|GetArrayItem` _nearby_pickup_actors))
  (if (and (`KismetSystemLibrary.IsValid` _output) (!= _output self))
    (`SceneComponent.SetVisibility` (`self.Pickup Text`) false false)
    (`KismetArrayLibrary.Array_RemoveItem` _nearby_pickup_actors self)
    (bind _output_2 (`|GetArrayItem` _nearby_pickup_actors))
    (`/Engine/EditorBlueprintResources/StandardMacros.IsValid` _output_2
      (:`Is Valid`
        (`SceneComponent.SetVisibility` (`/Game/BluePrints/Game_Settings/Items/Inventory_System/Blueprints/ItemClasses/BP_PickupActor.Pickup Text` _output_2) true false)))
    (else
      (`KismetArrayLibrary.Array_RemoveItem` _nearby_pickup_actors self))))

(fn `Random Amount to Add`
  (params (`Min Amount` :type Integer) (`Max Amount` :type Integer))
  (returns (`Amount to Add` :type Integer))
  (return (`KismetMathLibrary.RandomIntegerInRange` `Min Amount` `Max Amount`)))

(fn `Update Text`
  (bind _aswb_pickup_text (cast `/Game/BluePrints/Game_Settings/Items/Inventory_System/Widgets/WB_PickupText` (`WidgetComponent.GetUserWidgetObject` (`self.Pickup Text`)))
    (:`then`
      (`TextBlock.SetText` (`/Game/BluePrints/Game_Settings/Items/Inventory_System/Widgets/WB_PickupText.NameText` _aswb_pickup_text) (`|FormatText` "{Name} {Amount}" (`.Name_2_D31A47854865B9CD63D753A5010406B0` (break `/Game/BluePrints/Game_Settings/Items/Inventory_System/Blueprints/Structures/S_ItemInfo` (defaults `/Game/BluePrints/Game_Settings/Items/Inventory_System/Blueprints/ItemClasses/BP_PickupActor` (`self.Item To Add`)))) (`KismetTextLibrary.Conv_IntToText` (`self.Amount`)))))
    (:`CastFailed`
      (`KismetSystemLibrary.PrintString` "failed - pickup actor-")))
  (return))

(fn `UserConstructionScript`
  (bind _item_to_add (`self.Item To Add`))
  (bind _static_mesh (`self.Static Mesh`))
  (bind (_name _description _icon _canbeused_ _usetext _canbestacked_ _category _pickupmesh _meshscale _interactradius) (break `/Game/BluePrints/Game_Settings/Items/Inventory_System/Blueprints/Structures/S_ItemInfo` (defaults `/Game/BluePrints/Game_Settings/Items/Inventory_System/Blueprints/ItemClasses/BP_PickupActor` _item_to_add)))
  (if (`KismetSystemLibrary.IsValidClass` _item_to_add)
    (`StaticMeshComponent.SetStaticMesh` _static_mesh _pickupmesh)
    (`SceneComponent.SetRelativeScale3D` _static_mesh _meshscale)
    (`SphereComponent.SetSphereRadius` (`self.Sphere`) _interactradius false)))