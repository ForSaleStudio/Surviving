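; BP_Ammo is an inventory item class that supplies ammo to the character's equipped weapon when used.
; Its used event proceeds only if current ammo does not exceed max ammo and max ammo is below the weapon's default maximum.
; It then passes the weapon's reload amount to the character's UseAmmo, removes that same amount from its inventory slot and destroys itself.
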(event `self.Event On Used`
  (bind _character_ref (`/Game/BluePrints/Game_Settings/Items/Inventory_System/Blueprints/BP_Inventory.Character Ref` (`self.Inventory Ref`)))
  (bind _equipped_weapon (`/Game/BluePrints/Game_Settings/Characters/Main_Characters/DR_Main_Character_base.Equipped Weapon` _character_ref))
  (bind _reload_ammo (`/Game/BluePrints/Game_Settings/Weapons/PrimaryWeapons/DR_Weapon_Base.Reload Ammo` _equipped_weapon))
  (bind _max_ammo (`/Game/BluePrints/Game_Settings/Weapons/PrimaryWeapons/DR_Weapon_Base.Max Ammo` _equipped_weapon))
  (if (and (<= (`/Game/BluePrints/Game_Settings/Weapons/PrimaryWeapons/DR_Weapon_Base.Cur Ammo` _equipped_weapon) _max_ammo) (< _max_ammo (`/Game/BluePrints/Game_Settings/Weapons/PrimaryWeapons/DR_Weapon_Base.Default Max Ammo` _equipped_weapon)))
    (`/Game/BluePrints/Game_Settings/Characters/Main_Characters/DR_Main_Character_base.Use Ammo` _character_ref _reload_ammo)
    (`/Game/BluePrints/Game_Settings/Items/Inventory_System/Blueprints/BP_Inventory.Remove Item At Index` (`self.Inventory Ref`) (`self.Index`) _reload_ammo)
    (`self.K2_DestroyActor`)))

(fn `UserConstructionScript`
  (`parent.UserConstructionScript`))