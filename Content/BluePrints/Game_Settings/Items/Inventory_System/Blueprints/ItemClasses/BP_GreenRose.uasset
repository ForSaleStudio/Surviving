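; BP_GreenRose is a usable inventory item that kills nearby AI enemies with an expanding area effect.
; On use it removes one from the inventory, then a timeline grows its detection sphere and the actor destroys itself after a short delay.
; Any DR_AI_CharacterBase that begins overlapping the sphere is flagged dead and receives damage.
; An unconnected draft for spawning the rose at the character's item spawn point never runs.
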(event `self.Event On Used`
  ;[0.001522 0.1354 0.02737] Changing the Sphere Radius on the rose for detecting enemies in its radius.
  (`/Game/BluePrints/Game_Settings/Items/Inventory_System/Blueprints/BP_Inventory.Remove Item At Index` (`self.Inventory Ref`) (`self.Index`) 1)
  (bind (_direction _increase_radius) (`Timeline|Sphere Change`)
    (:`Update`
      (`SphereComponent.SetSphereRadius` (`self.Detection Sphere`) (* 480 _increase_radius) true))
    (:`Finished`
      (`KismetSystemLibrary.Delay` 2.0)
      (`self.K2_DestroyActor`))))

(event `self.Detection Sphere.OnComponentBeginOverlap`
  (params (OverlappedComponent :type "PrimitiveComponent Object Reference") (OtherActor :type "Actor Object Reference") (OtherComp :type "PrimitiveComponent Object Reference") (OtherBodyIndex :type Integer) (bFromSweep :type Boolean) (SweepResult :type "HitResult Structure (by ref)"))
  ;[0.001522 0.1354 0.02737] Detecting if any of the enemies comes into contact with the sphere, then kills them.
  (bind _asdr_ai_character_base (cast `/Game/BluePrints/Game_Settings/Characters/Main_Enemies/Artificial_Intelligence/DR_AI_CharacterBase` OtherActor))
  (set `/Game/BluePrints/Game_Settings/Characters/Main_Enemies/Artificial_Intelligence/DR_AI_CharacterBase.Is Dead?` true _asdr_ai_character_base)
  (`GameplayStatics.ApplyDamage` _asdr_ai_character_base 100.0))

(fn `UserConstructionScript`
  (`parent.UserConstructionScript`))