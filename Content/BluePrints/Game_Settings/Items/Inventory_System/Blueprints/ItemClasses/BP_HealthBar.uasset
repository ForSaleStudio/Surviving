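; BP_HealthBar is a consumable inventory item class that restores some of the owning character's health when used.
; On use, it checks through its inventory reference whether health is below maximum, and if so increases health slightly and removes one unit from its slot.
; The actor destroys itself either way, so at full health nothing is healed or removed from the inventory.
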(event `self.Event On Used`
  (bind _character_ref (`/Game/BluePrints/Game_Settings/Items/Inventory_System/Blueprints/BP_Inventory.Character Ref` (`self.Inventory Ref`)))
  (if (< (`/Game/BluePrints/Game_Settings/Characters/Main_Characters/DR_Main_Character_base.Character Health` _character_ref) (`/Game/BluePrints/Game_Settings/Characters/Main_Characters/DR_Main_Character_base.Character Max Health` _character_ref))
    (`/Game/BluePrints/Game_Settings/Characters/Main_Characters/DR_Main_Character_base.Increase Health` _character_ref 0.1)
    (`/Game/BluePrints/Game_Settings/Items/Inventory_System/Blueprints/BP_Inventory.Remove Item At Index` (`self.Inventory Ref`) (`self.Index`) 1)
    (`self.K2_DestroyActor`)
    (else
      (`self.K2_DestroyActor`))))

(fn `UserConstructionScript`
  (`parent.UserConstructionScript`))