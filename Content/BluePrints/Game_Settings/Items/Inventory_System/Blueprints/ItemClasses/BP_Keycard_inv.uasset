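; Inventory keycard item that opens a keycard screen when used and is consumed once read.
; Using it disables the inventory widget, adds a WB_Keycard widget holding a reference to this actor at the center of the main inventory canvas, and switches input to UI only.
; OnRead re-enables the inventory, removes the keycard widget, restores game-and-UI input and destroys the actor.
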(event `self.Event On Used`
  (`Widget.SetIsEnabled` (`/Game/BluePrints/Game_Settings/Items/Inventory_System/Widgets/WB_MainInventoryWidget.InventoryWidget` (`/Game/BluePrints/Game_Settings/Items/Inventory_System/Blueprints/BP_Inventory.WB Main Inventory` (`self.Inventory Ref`))) false)
  (bind _returnvalue (`|CreateWidget` "/Game/BluePrints/Game_Settings/Items/Inventory_System/Widgets/WB_Keycard.WB_Keycard_C" null self))
  (bind _output_get (set `self.Keycard Widget` _returnvalue))
  (bind _returnvalue_2 (`CanvasPanel.AddChildToCanvas` (`/Game/BluePrints/Game_Settings/Items/Inventory_System/Widgets/WB_MainInventoryWidget.Canvas` (`/Game/BluePrints/Game_Settings/Items/Inventory_System/Blueprints/BP_Inventory.WB Main Inventory` (`self.Inventory Ref`))) _output_get))
  (`CanvasPanelSlot.SetAnchors` _returnvalue_2 (make `Anchors` (0.5 0.5) (0.5 0.5)))
  (`CanvasPanelSlot.SetAutoSize` _returnvalue_2 true)
  (`CanvasPanelSlot.SetPosition` _returnvalue_2 (-325.0 -240.0))
  (`WidgetBlueprintLibrary.SetInputMode_UIOnlyEx` (`GameplayStatics.GetPlayerController` 0) (`self.Keycard Widget`)))

(event `On Read`
  (`Widget.SetIsEnabled` (`/Game/BluePrints/Game_Settings/Items/Inventory_System/Widgets/WB_MainInventoryWidget.InventoryWidget` (`/Game/BluePrints/Game_Settings/Items/Inventory_System/Blueprints/BP_Inventory.WB Main Inventory` (`self.Inventory Ref`))) true)
  (`Widget.RemoveFromParent` (`self.Keycard Widget`))
  (`WidgetBlueprintLibrary.SetInputMode_GameAndUIEx` (`GameplayStatics.GetPlayerController` 0))
  (`self.K2_DestroyActor`))

(fn `UserConstructionScript`
  (`parent.UserConstructionScript`))