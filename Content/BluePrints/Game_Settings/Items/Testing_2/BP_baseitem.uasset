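; Base pickup item actor that adds itself to the main character's inventory when stepped on.
; Overlap of its pickup radius casts to DR_Main_Character_base, fills an item description struct with its name and image, appends it to NumInventory and destroys itself.
; An Activate event only prints the passed string in green as a placeholder for item use.
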(event `self.PickUp Radius.OnComponentBeginOverlap`
  (params (OverlappedComponent :type "PrimitiveComponent Object Reference") (OtherActor :type "Actor Object Reference") (OtherComp :type "PrimitiveComponent Object Reference") (OtherBodyIndex :type Integer) (bFromSweep :type Boolean) (SweepResult :type "HitResult Structure (by ref)"))
  ;[0.001522 0.1354 0.02737] Picking up the Item and added it to the inventory of the player.
  (bind _asdr_main_character_base (cast `/Game/BluePrints/Game_Settings/Characters/Main_Characters/DR_Main_Character_base` OtherActor))
  (bind _output_get (set `self.Main Character Ref` _asdr_main_character_base))
  (bind _structout (setmembers `/Game/BluePrints/Game_Settings/Items/Testing_2/Item_Desc` :`StructRef` (`self.Item Desc Ref`) :`Name` (`self.Item Name`) :`Image` (`self.Item Image`)))
  (`KismetArrayLibrary.Array_Add` (`/Game/BluePrints/Game_Settings/Characters/Main_Characters/DR_Main_Character_base.Num Inventory` _output_get) _structout)
  (`KismetSystemLibrary.PrintString` "Stepped on")
  (`self.K2_DestroyActor`))

(event `Activate`
  (params (sting :type String))
  (`KismetSystemLibrary.PrintString` sting true true (struct :`R` 0.001522 :`G` 0.135417 :`B` 0.027371 :`A` 1.0)))

(fn `UserConstructionScript`)