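; BP_ItemBase is a base item Blueprint that detects when the main character enters its pickup radius.
; On overlap it casts the other actor to DR_Main_Character_base and stores the reference.
; It copies the name and image from its item description struct into variables, writes them back into the same struct, and prints the item name.
; It does not add the item to an inventory or destroy itself.
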(event `self.PickUp Radius.OnComponentBeginOverlap`
  (params (OverlappedComponent :type "PrimitiveComponent Object Reference") (OtherActor :type "Actor Object Reference") (OtherComp :type "PrimitiveComponent Object Reference") (OtherBodyIndex :type Integer) (bFromSweep :type Boolean) (SweepResult :type "HitResult Structure (by ref)"))
  (bind _item_desc_ref (`self.Item Desc Ref`))
  (bind (_name _image) (break `/Game/BluePrints/Game_Settings/Items/Testing_2/Item_Desc` (`self.Item Desc Ref`)))
  (bind _asdr_main_character_base (cast `/Game/BluePrints/Game_Settings/Characters/Main_Characters/DR_Main_Character_base` OtherActor))
  (set `self.Main Character Ref` _asdr_main_character_base)
  (set `self.Item Name` _name)
  (set `self.Item Image` _image)
  (setmembers `/Game/BluePrints/Game_Settings/Items/Testing_2/Item_Desc` :`StructRef` _item_desc_ref :`Name` (`self.Item Name`) :`Image` (`self.Item Image`))
  (`KismetSystemLibrary.PrintString` (`KismetTextLibrary.Conv_TextToString` (`.Name_3_6F44858748F8088CCA4685B1483E7C93` (break `/Game/BluePrints/Game_Settings/Items/Testing_2/Item_Desc` _item_desc_ref)))))

(fn `UserConstructionScript`)