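; Test player controller for gamepad-driven UI navigation, which shows the mouse cursor and opens the Testing widget in Game and UI input mode on BeginPlay.
; Shoulder buttons and D-pad up/down send enum-coded navigation requests to that widget.
; Holding D-pad up or down repeats the request through a looping half-second timer, cleared on release.
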(event `self.ReceiveBeginPlay`
  (set `self.bShowMouseCursor` true)
  (bind _returnvalue (`|CreateWidget` "/Game/BluePrints/UserInterfaces/Testing.Testing_C"))
  (bind _output_get (set `self.MainWidget` _returnvalue))
  (`UserWidget.AddToViewport` _output_get 0)
  (`WidgetBlueprintLibrary.SetInputMode_GameAndUIEx` self (`self.MainWidget`)))

(event `Key|Gamepad_RightShoulder`
  (params (Key :type "Key Structure"))
  (:`Pressed`
    (`/Game/BluePrints/UserInterfaces/Testing.ReceiveNavigationRequest` (`self.MainWidget`) "NewEnumerator1")))

(event `Key|Gamepad_LeftShoulder`
  (params (Key :type "Key Structure"))
  (:`Pressed`
    (`/Game/BluePrints/UserInterfaces/Testing.ReceiveNavigationRequest` (`self.MainWidget`) "NewEnumerator0")))

(event `Key|Gamepad_DPad_Up`
  (params (Key :type "Key Structure"))
  (:`Pressed`
    (`self.GoUp`)
    (bind _returnvalue (`KismetSystemLibrary.K2_SetTimerDelegate` (delegate `GoUp`) 0.5 true))
    (set `self.DPadUp_Timer` _returnvalue))
  (:`Released`
    (`KismetSystemLibrary.K2_ClearAndInvalidateTimerHandle` (`self.DPadUp_Timer`))))

(event `GoUp`
  (`/Game/BluePrints/UserInterfaces/Testing.ReceiveNavigationRequest` (`self.MainWidget`) "NewEnumerator2"))

(event `Key|Gamepad_DPad_Down`
  (params (Key :type "Key Structure"))
  (:`Pressed`
    (`self.GoDown`)
    (bind _returnvalue (`KismetSystemLibrary.K2_SetTimerDelegate` (delegate `GoDown`) 0.5 true))
    (set `self.DPadDown_Timer` _returnvalue))
  (:`Released`
    (`KismetSystemLibrary.K2_ClearAndInvalidateTimerHandle` (`self.DPadDown_Timer`))))

(event `GoDown`
  (`/Game/BluePrints/UserInterfaces/Testing.ReceiveNavigationRequest` (`self.MainWidget`) "NewEnumerator3"))

(fn `UserConstructionScript`)