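; Base projectile Blueprint that damages AI characters it overlaps.
; When BulletCollision begins an overlap, it casts the other actor to DR_AI_CharacterBase and applies its Damage value through ApplyDamage.
; Debug prints report the damage value at BeginPlay, the damage taken on a hit, and failed casts.
; The graph contains no movement or destroy logic, and the construction script is empty.
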(event `self.ReceiveBeginPlay`
  (`KismetSystemLibrary.PrintString` (`KismetStringLibrary.Concat_StrStr` "Weapon Damage at: " (`KismetStringLibrary.Conv_DoubleToString` (`self.Damage`)))))

(event `self.Bullet Collision.OnComponentBeginOverlap`
  (params (OverlappedComponent :type "PrimitiveComponent Object Reference") (OtherActor :type "Actor Object Reference") (OtherComp :type "PrimitiveComponent Object Reference") (OtherBodyIndex :type Integer) (bFromSweep :type Boolean) (SweepResult :type "HitResult Structure (by ref)"))
  (bind _asdr_ai_character_base (cast `/Game/BluePrints/Game_Settings/Characters/Main_Enemies/Artificial_Intelligence/DR_AI_CharacterBase` OtherActor)
    (:`then`
      (bind _returnvalue (`GameplayStatics.ApplyDamage` _asdr_ai_character_base (`self.Damage`)))
      (`KismetSystemLibrary.PrintString` (`KismetStringLibrary.Concat_StrStr` "AI has taken " (`KismetStringLibrary.Conv_DoubleToString` _returnvalue) " points of damage.") true true (struct :`R` 0.029894 :`G` 0.124372 :`B` 0.302083 :`A` 1.0) 2.0))
    (:`CastFailed`
      (`KismetSystemLibrary.PrintString` "cast failed -projectile-"))))

(fn `UserConstructionScript`)