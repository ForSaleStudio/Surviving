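; BP_JailDoor_Test is a test double sliding jail door that opens when something overlaps its box trigger and closes when the overlap ends.
; BeginPlay stores each door's world start location and derives end points by shifting the two doors in opposite directions by configurable X and Y offsets.
; The OpenDoor timeline plays or reverses on overlap, lerping both doors between those points.
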(event `self.Test_Box.OnComponentBeginOverlap`
  (params (OverlappedComponent :type "PrimitiveComponent Object Reference") (OtherActor :type "Actor Object Reference") (OtherComp :type "PrimitiveComponent Object Reference") (OtherBodyIndex :type Integer) (bFromSweep :type Boolean) (SweepResult :type "HitResult Structure (by ref)"))
  (bind (_direction _newtrack_0) (`Timeline|Open Door` :!label _label)
    (:`Update`
      (`SceneComponent.K2_SetWorldLocation` (`self.TestDoor`) (`KismetMathLibrary.VLerp` (`self.Door Start`) (`self.Door End`) _newtrack_0) false false)
      (`SceneComponent.K2_SetWorldLocation` (`self.TestDoor2`) (`KismetMathLibrary.VLerp` (`self.Door Start2`) (`self.Door End2`) _newtrack_0) false false))))

(event `self.Test_Box.OnComponentEndOverlap`
  (params (OverlappedComponent :type "PrimitiveComponent Object Reference") (OtherActor :type "Actor Object Reference") (OtherComp :type "PrimitiveComponent Object Reference") (OtherBodyIndex :type Integer))
  (goto _label :!via `Reverse`))

(event `self.ReceiveBeginPlay`
  (bind _returnvalue (`SceneComponent.K2_GetComponentLocation` (`self.TestDoor`)))
  (bind _returnvalue_2 (`SceneComponent.K2_GetComponentLocation` (`self.TestDoor2`)))
  (set `self.Door Start` _returnvalue)
  (set `self.Door End` (`KismetMathLibrary.MakeVector` (+ (.x _returnvalue) (`self.Offset X`)) (+ (.y _returnvalue) (`self.Offset Y`)) (.z _returnvalue)))
  (set `self.Door Start2` _returnvalue_2)
  (set `self.Door End2` (`KismetMathLibrary.MakeVector` (- (.x _returnvalue_2) (`self.Offset X`)) (- (.y _returnvalue_2) (`self.Offset Y`)) (.z _returnvalue_2))))

(fn `UserConstructionScript`)