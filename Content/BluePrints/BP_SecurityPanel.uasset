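; Security panel Blueprint that lets the player enter a password on a keypad to open a linked door.
; UseKeypad creates the DR_Keypad widget, passes it a reference to the panel, and switches the player to UI-only input with a visible cursor.
; CorrectPassword calls OpenDoor on the referenced DoorBP; the panel itself holds no password check.
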(event `Use Keypad`
  (bind _returnvalue (`GameplayStatics.GetPlayerController` 0))
  (bind _returnvalue_2 (`|CreateWidget` "/Game/BluePrints/UserInterfaces/DR_Keypad.DR_Keypad_C"))
  (set `/Game/BluePrints/UserInterfaces/DR_Keypad.BP_SecurityPanel` self _returnvalue_2)
  (`UserWidget.AddToViewport` _returnvalue_2 0)
  (`WidgetBlueprintLibrary.SetInputMode_UIOnlyEx` _returnvalue _returnvalue_2)
  (set `PlayerController.bShowMouseCursor` true _returnvalue)
  (`KismetSystemLibrary.PrintString` "Hello"))

(event `Correct Password`
  (`/Game/BluePrints/Interactables/BP_Door_test.Open Door` (`self.DoorBP`)))

(fn `UserConstructionScript`)