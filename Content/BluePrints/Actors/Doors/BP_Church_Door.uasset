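; Church door actor that toggles open or closed when the main character or a cine camera begins overlapping its collision box.
; The Open timeline lerps FrontFacingArrow's relative rotation through 90 degrees, playing from start to open and reversing from end to close.
; IsOpen flips only when the timeline finishes, so an overlap mid-swing restarts the same motion.
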(event `Open Door`
  (bind (_direction _open) (`Timeline|Open` :!via `PlayFromStart` :!label _label)
    (:`Update`
      (`SceneComponent.K2_SetRelativeRotation` (`self.Front Facing Arrow`) (`KismetMathLibrary.RLerp` (struct) (struct :`Yaw` 90.0) _open) false false))
    (:`Finished`
      (if (`self.Is Open?`)
        (set `self.Is Open?` false)
        (else
          (set `self.Is Open?` true))))))

(event `Close Door`
  (goto _label :!via `ReverseFromEnd`))

(event `self.Collision Box.OnComponentBeginOverlap`
  (params (OverlappedComponent :type "PrimitiveComponent Object Reference") (OtherActor :type "Actor Object Reference") (OtherComp :type "PrimitiveComponent Object Reference") (OtherBodyIndex :type Integer) (bFromSweep :type Boolean) (SweepResult :type "HitResult Structure (by ref)"))
  (cast `/Game/BluePrints/Game_Settings/Characters/Main_Characters/DR_Main_Character_base` OtherActor
    (:`then`
      _)
    (:`CastFailed`
      (cast `CineCameraActor` OtherActor)))
  (if (`self.Is Open?`)
    (`self.Close Door`)
    (else
      (`self.Open Door`))))

(fn `UserConstructionScript`)