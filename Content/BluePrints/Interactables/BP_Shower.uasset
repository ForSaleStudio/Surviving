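; BP_Shower is an interactable shower whose particle effect the player can toggle on and off.
; Overlapping its box creates a DR_Interactable prompt widget and enables input; leaving disables input and removes the widget.
; E or the gamepad left face button toggles the particle system's visibility and flips IsOn.
; The effect is only hidden, never deactivated, as the Deactivate call is unconnected.
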(event `Key|Gamepad_FaceButton_Left`
  (params (Key :type "Key Structure"))
  ;[1 1 1] Toggling the Shower Scene
  (:`Pressed`
    (if (`self.Is On?`) :!label _label
      (`SceneComponent.ToggleVisibility` (`self.ParticleSystem`) false)
      (set `self.Is On?` false)
      (else
        (`SceneComponent.ToggleVisibility` (`self.ParticleSystem`) false)
        (set `self.Is On?` true)))))

(event `self.Box.OnComponentBeginOverlap`
  (params (OverlappedComponent :type "PrimitiveComponent Object Reference") (OtherActor :type "Actor Object Reference") (OtherComp :type "PrimitiveComponent Object Reference") (OtherBodyIndex :type Integer) (bFromSweep :type Boolean) (SweepResult :type "HitResult Structure (by ref)"))
  (bind _returnvalue (`GameplayStatics.GetPlayerController` 0))
  ;[1 1 1] Enabling the user to Toggle the Shower
  (bind _returnvalue_2 (`|CreateWidget` "/Game/BluePrints/UserInterfaces/DR_Interactable.DR_Interactable_C" _returnvalue))
  (`UserWidget.AddToViewport` _returnvalue_2 0)
  (`self.EnableInput` _returnvalue))

(event `Key|E`
  (params (Key :type "Key Structure"))
  ;[1 1 1] Toggling the Shower Scene
  (:`Pressed`
    (goto _label)))

(event `self.Box.OnComponentEndOverlap`
  (params (OverlappedComponent :type "PrimitiveComponent Object Reference") (OtherActor :type "Actor Object Reference") (OtherComp :type "PrimitiveComponent Object Reference") (OtherBodyIndex :type Integer))
  ;[1 1 1] Enabling the user to Toggle the Shower
  (`self.DisableInput` (`GameplayStatics.GetPlayerController` 0))
  (`Widget.RemoveFromParent` (stale `self.Box.OnComponentBeginOverlap` _returnvalue_2)))

(fn `UserConstructionScript`)