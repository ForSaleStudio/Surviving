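; Keycard-locked door that swings open when the player's card matches the required one, is the master card, or no card is required.
; An outer reader overlap checks the character's keycard, drives granted or denied sound and keypad widget feedback, then opens after a delay or closes.
; An inner box toggles the door without a card check.
; A timeline lerps the Arrow component's rotation, reversing to close.
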(event `self.ReceiveBeginPlay`
  ;[1 1 1] Checking to see if there is no keycard required.
  (set `self.No Key` (`|EnumEquality` (`self.Required Keycard`) "NewEnumerator4")))

(event `Set Sound`
  (bind _access_audio (`self.Access Audio`))
  ;[1 1 1] Setting the proper sounds to be heard
  (switch `/Game/Sounds/Enum_Keycard_Sounds` (`self.Access Sound`)
    (:`NewEnumerator0`
      (bind _output_get (set `self.Keypad Sound` "/Game/Sounds/access_granted_test.access_granted_test"))
      (`AudioComponent.SetSound` _access_audio _output_get))
    (:`NewEnumerator4`
      (bind _output_get_2 (set `self.Keypad Sound` "/Game/Sounds/Access_Denied_keyM_test.Access_Denied_keyM_test"))
      (`AudioComponent.SetSound` _access_audio _output_get_2))
    (:`NewEnumerator1`
      (bind _output_get_3 (set `self.Keypad Sound` "/Game/Sounds/Access_Denied_keyA_test.Access_Denied_keyA_test"))
      (`AudioComponent.SetSound` _access_audio _output_get_3))
    (:`NewEnumerator2`
      (bind _output_get_4 (set `self.Keypad Sound` "/Game/Sounds/Access_Denied_keyB_test.Access_Denied_keyB_test"))
      (`AudioComponent.SetSound` _access_audio _output_get_4))
    (:`NewEnumerator3`
      (bind _output_get_5 (set `self.Keypad Sound` "/Game/Sounds/Access_Denied_keyC_test.Access_Denied_keyC_test"))
      (`AudioComponent.SetSound` _access_audio _output_get_5))))

(event `Open Door`
  ;[1 1 1] Door opening / closing animation
  (bind (_direction _open_door) (`Timeline|Door Open Animation` :!label _label)
    (:`Update`
      (`SceneComponent.K2_SetRelativeRotation` (`self.Arrow`) (`KismetMathLibrary.RLerp` (struct) (struct :`Yaw` 90.0) _open_door) false false))))

(event `Close Door`
  ;[1 1 1] Door opening / closing animation
  (goto _label :!via `Reverse`))

(event `self.Keycard Reader Box2.OnComponentBeginOverlap`
  (params (OverlappedComponent :type "PrimitiveComponent Object Reference") (OtherActor :type "Actor Object Reference") (OtherComp :type "PrimitiveComponent Object Reference") (OtherBodyIndex :type Integer) (bFromSweep :type Boolean) (SweepResult :type "HitResult Structure (by ref)"))
  ;[1 1 1] Closing the doors from the inside.
  (if (`self.Is Door Open?`)
    (`self.Close Door`)
    (set `self.Is Door Open?` false)
    (else
      (`self.Open Door`))))

(event `self.Keycard Reader Box.OnComponentBeginOverlap`
  (params (OverlappedComponent :type "PrimitiveComponent Object Reference") (OtherActor :type "Actor Object Reference") (OtherComp :type "PrimitiveComponent Object Reference") (OtherBodyIndex :type Integer) (bFromSweep :type Boolean) (SweepResult :type "HitResult Structure (by ref)"))
  (bind _returnvalue (`WidgetComponent.GetUserWidgetObject` (`self.KeycardScreen`)))
  ;[1 1 1] Everything that makes the doors do their things....
  (bind _asdr_main_character_base (cast `/Game/BluePrints/Game_Settings/Characters/Main_Characters/DR_Main_Character_base` OtherActor))
  (bind _keycards (`/Game/BluePrints/Game_Settings/Characters/Main_Characters/DR_Main_Character_base.Keycards` _asdr_main_character_base))
  (set `self.Mastercard` (`|EnumEquality` _keycards "NewEnumerator0"))
  (if (or (`self.Mastercard`) (`self.Is Door Open?`) (`self.No Key`) (`|EnumEquality` (`self.Required Keycard`) _keycards))
    (set `self.Is Door Open?` true)
    (set `self.Access Sound` "NewEnumerator0")
    (`self.Set Sound`)
    (bind _asdr_wb_keypad_color (cast `/Game/BluePrints/UserInterfaces/Interactables_Widgets/DR_WB_KeypadColor` _returnvalue))
    (if (not (`self.Has Sound Played?`))
      (`GameplayStatics.PlaySoundAtLocation` (`self.Keypad Sound`) (`SceneComponent.K2_GetComponentLocation` (`self.Access Audio`)))
      (set `self.Has Sound Played?` true))
    (`/Game/BluePrints/UserInterfaces/Interactables_Widgets/DR_WB_KeypadColor.Access Granted` _asdr_wb_keypad_color)
    (`KismetSystemLibrary.Delay` 2.0)
    (`self.Open Door`)
    (else
      (`self.Set Sound`)
      (bind _asdr_wb_keypad_color_2 (cast `/Game/BluePrints/UserInterfaces/Interactables_Widgets/DR_WB_KeypadColor` _returnvalue))
      (`GameplayStatics.PlaySoundAtLocation` (`self.Keypad Sound`) (`SceneComponent.K2_GetComponentLocation` (`self.Access Audio`)))
      (`/Game/BluePrints/UserInterfaces/Interactables_Widgets/DR_WB_KeypadColor.Access Denied` _asdr_wb_keypad_color_2)
      (`self.Close Door`))))

(fn `UserConstructionScript`)