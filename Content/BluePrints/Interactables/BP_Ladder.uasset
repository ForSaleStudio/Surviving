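; BP_Ladder is an interactable ladder that tells the main character when it is within climbing range.
; Entering its Box trigger creates an interaction prompt widget for player 0 and sets the character's IsNearLadder flag.
; Leaving clears the near-ladder and on-ladder flags, restores Walking movement and removes the prompt.
; The climbing movement itself is not handled in this Blueprint.
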(event `self.Box.OnComponentBeginOverlap`
  (params (OverlappedComponent :type "PrimitiveComponent Object Reference") (OtherActor :type "Actor Object Reference") (OtherComp :type "PrimitiveComponent Object Reference") (OtherBodyIndex :type Integer) (bFromSweep :type Boolean) (SweepResult :type "HitResult Structure (by ref)"))
  (bind _asdr_main_character_base (cast `/Game/BluePrints/Game_Settings/Characters/DR_Main_Character_base` OtherActor))
  ;[1 1 1] Creating the pop up to let the user know how to use the ladder
  (bind _returnvalue (`|CreateWidget` "/Game/BluePrints/UserInterfaces/Interactables_Widgets/DR_WB_Interactable.DR_WB_Interactable_C" (`GameplayStatics.GetPlayerController` 0)))
  (`UserWidget.AddToViewport` _returnvalue 0)
  (set `/Game/BluePrints/Game_Settings/Characters/DR_Main_Character_base.Is Near Ladder` true _asdr_main_character_base))

(event `self.Box.OnComponentEndOverlap`
  (params (OverlappedComponent :type "PrimitiveComponent Object Reference") (OtherActor :type "Actor Object Reference") (OtherComp :type "PrimitiveComponent Object Reference") (OtherBodyIndex :type Integer))
  (bind _asdr_main_character_base (cast `/Game/BluePrints/Game_Settings/Characters/DR_Main_Character_base` OtherActor))
  (set `/Game/BluePrints/Game_Settings/Characters/DR_Main_Character_base.Is Near Ladder` false _asdr_main_character_base)
  (set `/Game/BluePrints/Game_Settings/Characters/DR_Main_Character_base.Is On Ladder` false _asdr_main_character_base)
  (`CharacterMovementComponent.SetMovementMode` (`Character.CharacterMovement` _asdr_main_character_base) "MOVE_Walking" 0)
  (`Widget.RemoveFromParent` (stale `self.Box.OnComponentBeginOverlap` _returnvalue)))

(fn `UserConstructionScript`)