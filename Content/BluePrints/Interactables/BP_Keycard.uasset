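; BP_Keycard is a pickup that gives the player a keycard when something overlaps its box.
; On overlap it casts player character 0 to DR_Main_Character_base, sets that character's Keycards value to this card's Keycard enum, then destroys itself.
; The value is assigned rather than added, and the overlapping actor is never checked.
; Debug prints show its location at BeginPlay and the keycard on pickup.
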(event `self.ReceiveBeginPlay`
  (`KismetSystemLibrary.PrintString` (`KismetStringLibrary.Conv_VectorToString` (`self.K2_GetActorLocation`)) true true (struct :`G` 0.66 :`B` 1.0 :`A` 1.0) 10.0))

(event `self.Box.OnComponentBeginOverlap`
  (params (OverlappedComponent :type "PrimitiveComponent Object Reference") (OtherActor :type "Actor Object Reference") (OtherComp :type "PrimitiveComponent Object Reference") (OtherBodyIndex :type Integer) (bFromSweep :type Boolean) (SweepResult :type "HitResult Structure (by ref)"))
  (bind _asdr_main_character_base (cast `/Game/BluePrints/Game_Settings/Characters/Main_Characters/DR_Main_Character_base` (`GameplayStatics.GetPlayerCharacter` 0)))
  (set `/Game/BluePrints/Game_Settings/Characters/Main_Characters/DR_Main_Character_base.Keycards` (`self.Keycard`) _asdr_main_character_base)
  (`self.K2_DestroyActor`)
  (`KismetSystemLibrary.PrintString` (`|GetEnumeratorNameAsString` (`self.Keycard`)))
  (`KismetSystemLibrary.PrintString` "should be the new keycard"))

(fn `UserConstructionScript`)