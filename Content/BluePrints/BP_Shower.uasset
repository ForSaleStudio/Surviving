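; BP_Shower is an interactive shower whose particle effect the player toggles while standing inside its box trigger.
; Box overlap begin and end enable and disable input for player controller 0, printing a debug message, with no check on the overlapping actor.
; E or the left gamepad face button flips the particle visibility and the IsOn flag; both branches make the same ToggleVisibility call, so the flag only tracks state.
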(event `self.Box.OnComponentBeginOverlap`
  (params (OverlappedComponent :type "PrimitiveComponent Object Reference") (OtherActor :type "Actor Object Reference") (OtherComp :type "PrimitiveComponent Object Reference") (OtherBodyIndex :type Integer) (bFromSweep :type Boolean) (SweepResult :type "HitResult Structure (by ref)"))
  ;[1 1 1] Enabling the user to Toggle the Shower
  (`KismetSystemLibrary.PrintString` "In box")
  (`self.EnableInput` (`GameplayStatics.GetPlayerController` 0)))

(event `Key|Gamepad_FaceButton_Left`
  (params (Key :type "Key Structure"))
  ;[1 1 1] Toggling the Shower Scene
  (:`Pressed`
    (if (`self.Is On?`) :!label _label
      (`SceneComponent.ToggleVisibility` (`self.ParticleSystem`) false)
      (set `self.Is On?` false)
      (else
        (`SceneComponent.ToggleVisibility` (`self.ParticleSystem`) false)
        (set `self.Is On?` true)))))

(event `Key|E`
  (params (Key :type "Key Structure"))
  ;[1 1 1] Toggling the Shower Scene
  (:`Pressed`
    (goto _label)))

(event `self.Box.OnComponentEndOverlap`
  (params (OverlappedComponent :type "PrimitiveComponent Object Reference") (OtherActor :type "Actor Object Reference") (OtherComp :type "PrimitiveComponent Object Reference") (OtherBodyIndex :type Integer))
  ;[1 1 1] Enabling the user to Toggle the Shower
  (`KismetSystemLibrary.PrintString` "Out Box")
  (`self.DisableInput` (`GameplayStatics.GetPlayerController` 0)))

(fn `UserConstructionScript`)