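; Minimap world capture actor that frames the level for an orthographic SceneCapture, using UpperLeft and LowerRight reference actors as bounds.
; The construction script moves it to the XY midpoint of the two references, keeping its own Z.
; It sets the capture's OrthoWidth to the larger of the X and Y spans, and runs no gameplay logic.
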(fn `UserConstructionScript`
  (bind _returnvalue (`self.K2_GetActorLocation` (`self.Upper Left`)))
  ;[0.001522 0.1354 0.02737] Getting the "Middle" of the map by doing math (b/w the upper left point and lower right point).
  (`/Engine/EditorBlueprintResources/StandardMacros.IsValid` (`self.Upper Left`)
    (:`Is Valid`
      (`/Engine/EditorBlueprintResources/StandardMacros.IsValid` (`self.Lower Right`)
        (:`Is Valid`
          (`self.K2_SetActorLocation` (`KismetMathLibrary.MakeVector` (.x (+ _returnvalue (/ (- (`self.K2_GetActorLocation` (`self.Lower Right`)) _returnvalue) 2.0))) (.y (+ _returnvalue (/ (- (`self.K2_GetActorLocation` (`self.Lower Right`)) _returnvalue) 2.0))) (.z (`self.K2_GetActorLocation`))) false true)
          (set `SceneCaptureComponent2D.OrthoWidth` (`KismetMathLibrary.FMax` (`KismetMathLibrary.Abs` (- (.x (`self.K2_GetActorLocation` (`self.Lower Right`))) (.x (`self.K2_GetActorLocation` (`self.Upper Left`))))) (`KismetMathLibrary.Abs` (- (.y (`self.K2_GetActorLocation` (`self.Lower Right`))) (.y (`self.K2_GetActorLocation` (`self.Upper Left`)))))) (`self.Scene Capture`)))))))