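; World map component that shows the player's position and undiscovered areas on a toggleable UI map.
; On initialization it creates the main level widget and adds a scaled circle for each undiscovered area actor.
; World locations convert to widget positions relative to two corner actors; the player marker updates on movement while visible.
; Discovering an area removes its circle and notifies the area, while toggling visibility switches cursor and input mode.
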(event `Initialize Map`
  (params (Player :type "Character Object Reference"))
  (bind _map_ref (`self.Map Ref`))
  (`/Engine/EditorBlueprintResources/StandardMacros.IsValid` Player
    (:`Is Valid`
      (set `self.Player` Player)
      (`KismetSystemLibrary.PrintString` "Successful -bpc world map-" true true (struct :`R` 1.0 :`A` 1.0) 5.0)
      (bind _returnvalue (`|CreateWidget` "/Game/Levels/MiniMap/Widgets/WB_Lvl_Main.WB_Lvl_Main_C"))
      (bind _output_get (set `self.Main Ref` _returnvalue))
      (bind _output_get_2 (set `self.Map Ref` (`/Game/Levels/MiniMap/Widgets/WB_Lvl_Main.WorldMap` _output_get)))
      (`/Game/Levels/MiniMap/Widgets/WB_Lvl_WorldMap.Initialize` _output_get_2 self)
      (set `self.Original Player Size` (`KismetMathLibrary.MakeVector2D` (`KismetMathLibrary.Conv_IntToDouble` (`/Game/Levels/MiniMap/Widgets/WB_Lvl_WorldMap.Player Size X` _map_ref)) (`KismetMathLibrary.Conv_IntToDouble` (`/Game/Levels/MiniMap/Widgets/WB_Lvl_WorldMap.Player Size Y` _map_ref))))
      (bind _outactors (`GameplayStatics.GetAllActorsOfClass` "/Game/Levels/MiniMap/Actors/BP_Lvl_UndiscoveredArea.BP_Lvl_UndiscoveredArea_C"))
      (bind _output_get_3 (set `self.Undiscovered Areas` _outactors))
      (for _array_element _output_get_3
        (bind _size (`self.Area Radius to Map Circle Size` _array_element))
        (bind _out (`/Game/Levels/MiniMap/Widgets/WB_Lvl_WorldMap.Add Area to Map` (`self.Map Ref`) _size (`self.Location to Map Position` (`Actor.K2_GetActorLocation` _array_element) (`KismetMathLibrary.MakeVector2D` _size _size))))
        (`KismetArrayLibrary.Array_Add` (`self.Area Widgets`) _out))
      (`self.Show Map` false)
      (`UserWidget.AddToViewport` (`self.Main Ref`) 0))
    (:`Is Not Valid`
      (`KismetSystemLibrary.PrintString` "Error Player is not valid - BPc world map-" true true (struct :`R` 1.0 :`A` 1.0) 10.0))))

(event `On Player Moved`
  (if (`self.Visible?`)
    (`self.Update Player Position on Map`)))

(event `On Discovered Area`
  (params (Area :type "/Game/Levels/MiniMap/Actors/BP_Lvl_UndiscoveredArea Object Reference"))
  (bind _undiscovered_areas (`self.Undiscovered Areas`))
  (bind _output (`|GetArrayItem` (`self.Area Widgets`) (`self.Area Index`)))
  (if (`KismetArrayLibrary.Array_Contains` (`self.Undiscovered Areas`) Area)
    (bind _output_get (set `self.Area Index` (`KismetArrayLibrary.Array_Find` _undiscovered_areas Area)))
    (`KismetArrayLibrary.Array_Remove` _undiscovered_areas _output_get)
    (`/Engine/EditorBlueprintResources/StandardMacros.IsValid` _output
      (:`Is Valid`
        (`/Game/Levels/MiniMap/Widgets/WB_Lvl_UndiscoveredArea.Remove Widget` _output)
        (`KismetArrayLibrary.Array_Remove` (`self.Area Widgets`) (`self.Area Index`)))
      (:`Is Not Valid`
        _))
    (`/Game/Levels/MiniMap/Actors/BP_Lvl_UndiscoveredArea.On Discovered` Area)))

(fn `Area Radius to Map Circle Size`
  (params (Area :type "/Game/Levels/MiniMap/Actors/BP_Lvl_UndiscoveredArea Object Reference"))
  (returns (Size :type "Float (double-precision)"))
  (return (* (/ (* (`/Game/Levels/MiniMap/Actors/BP_Lvl_UndiscoveredArea.Area Radius` Area) 2.0) (`self.Get Map Width`)) (`KismetMathLibrary.Conv_IntToDouble` (`/Game/Levels/MiniMap/Widgets/WB_Lvl_WorldMap.Map Size X` (`self.Map Ref`))))))

(fn `Convert Location to Map Location`
  (params (Location :type "Vector Structure"))
  (returns (Out :type "Vector2D Structure"))
  (return (`KismetMathLibrary.MakeVector2D` (`KismetMathLibrary.Abs` (- (.y Location) (.y (`Actor.K2_GetActorLocation` (`self.Upper Left Corner`))))) (`KismetMathLibrary.Abs` (- (.x Location) (.x (`Actor.K2_GetActorLocation` (`self.Upper Left Corner`))))))))

(fn `Get Map Height`
  (returns (Out :type "Float (double-precision)"))
  (return (`KismetMathLibrary.Abs` (- (.x (`Actor.K2_GetActorLocation` (`self.Lower Right Corner`))) (.x (`Actor.K2_GetActorLocation` (`self.Upper Left Corner`)))))))

(fn `Get Map Width`
  (returns (Out :type "Float (double-precision)"))
  (return (`KismetMathLibrary.Abs` (- (.y (`Actor.K2_GetActorLocation` (`self.Lower Right Corner`))) (.y (`Actor.K2_GetActorLocation` (`self.Upper Left Corner`)))))))

(fn `Location to Map Position`
  (params (Location :type "Vector Structure") (`Widget Size` :type "Vector2D Structure"))
  (returns (Out :type "Vector2D Structure"))
  (bind (_x _y) (`KismetMathLibrary.BreakVector2D` `Widget Size`))
  (bind _map_ref (`self.Map Ref`))
  (bind (_x_2 _y_2) (`KismetMathLibrary.BreakVector2D` (`self.Convert Location to Map Location` Location)))
  (return (`KismetMathLibrary.MakeVector2D` (- (* (/ _x_2 (`self.Get Map Width`)) (`KismetMathLibrary.Conv_IntToDouble` (`/Game/Levels/MiniMap/Widgets/WB_Lvl_WorldMap.Map Size X` _map_ref))) (/ _x 2.0)) (- (* (/ _y_2 (`self.Get Map Height`)) (`KismetMathLibrary.Conv_IntToDouble` (`/Game/Levels/MiniMap/Widgets/WB_Lvl_WorldMap.Map Size Y` _map_ref))) (/ _y 2.0)))))

(fn `Show Map`
  (params (`Show?` :type Boolean))
  (bind _returnvalue (`GameplayStatics.GetPlayerController` 0))
  (bind _returnvalue_2 (`GameplayStatics.GetPlayerController` 0))
  (if (!= `Show?` (`self.Visible?`))
    (bind _output_get (set `self.Visible?` `Show?`))
    (if _output_get
      (`Widget.SetVisibility` (`self.Map Ref`) "SelfHitTestInvisible")
      (set `PlayerController.bShowMouseCursor` true _returnvalue_2)
      (`WidgetBlueprintLibrary.SetInputMode_GameAndUIEx` _returnvalue_2 (`self.Main Ref`) "DoNotLock" false) ; thi smight need to be changed to just UI
      (`self.Update Player Position on Map`)
      (return)
      (else
        (`Widget.SetVisibility` (`self.Map Ref`) "Hidden")
        (set `PlayerController.bShowMouseCursor` false _returnvalue)
        (`WidgetBlueprintLibrary.SetInputMode_GameOnly` _returnvalue)
        (return)))
    (else
      (return))))

(fn `Toggle Visibility`
  (`self.Show Map` (not (`self.Visible?`)))
  (return))

(fn `Update Player Position on Map`
  (`Widget.SetRenderTranslation` (`/Game/Levels/MiniMap/Widgets/WB_Lvl_WorldMap.PlayerBox` (`self.Map Ref`)) (`self.Location to Map Position` (`Actor.K2_GetActorLocation` (`self.Player`)) (`self.Original Player Size`)))
  (return))