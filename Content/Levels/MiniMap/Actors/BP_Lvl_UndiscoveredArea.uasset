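; BP_Lvl_UndiscoveredArea is a placed level actor marking a minimap area the player has not yet discovered.
; Its construction script sizes an area sphere from AreaRadius and a larger discover sphere that adds AdditionalDiscoverRadius.
; When an actor with a BPc_WorldMap component overlaps the discover sphere, it reports itself once via that component's OnDiscoveredArea.
; Its OnDiscovered event destroys the actor.
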(event `On Discovered`
  (`self.K2_DestroyActor`))

(event `self.Discover Sphere.OnComponentBeginOverlap`
  (params (OverlappedComponent :type "PrimitiveComponent Object Reference") (OtherActor :type "Actor Object Reference") (OtherComp :type "PrimitiveComponent Object Reference") (OtherBodyIndex :type Integer) (bFromSweep :type Boolean) (SweepResult :type "HitResult Structure (by ref)"))
  (bind _returnvalue (`self.GetComponentByClass` OtherActor "/Game/Levels/MiniMap/Actors/BPc_WorldMap.BPc_WorldMap_C"))
  (`/Engine/EditorBlueprintResources/StandardMacros.IsValid` _returnvalue
    (:`Is Valid`
      (`/Engine/EditorBlueprintResources/StandardMacros.DoOnce` false
        (:`Completed`
          (`/Game/Levels/MiniMap/Actors/BPc_WorldMap.On Discovered Area` _returnvalue self))))))

(fn `UserConstructionScript`
  (bind _area_radius (`self.Area Radius`))
  (`SphereComponent.SetSphereRadius` (`self.Area Sphere`) _area_radius false)
  (`SphereComponent.SetSphereRadius` (`self.Discover Sphere`) (+ _area_radius (`self.Additional Discover Radius`)) false))